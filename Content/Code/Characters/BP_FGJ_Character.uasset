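; Fighting-game character that moves on a 2D Y/Z plane with custom kinematics and turns to face its Opponent while grounded.
; Each HandleInput call, rather than Tick, runs one step: walk or jump input, collision, velocity integration with gravity and friction, then facing.
; FloorCollider overlaps handle landing on Floor-tagged components and pushing off other characters.
; GetState and SetState save and restore position, velocity and facing.
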(event EventBeginPlay)

(event Collision|EventActorBeginOverlap
  (params (OtherActor :type Actor%20Object%20Reference)))

(event EventTick
  (params (DeltaSeconds :type Float%20%28single-precision%29)))

(event EventHandleInput
  (params (currentInput :type U%20Player%20Input%20Struct%20Structure))
  (bind (_up _dwn _lft _rgt) (Utilities|Struct|BreakUPlayerInputStruct currentInput))
  (bind _air_resistance (Variables|Default|GetAir%20Resistance))
  (Utilities|FlowControl|Sequence
    (:then_0
      ;[1 1 1] Inputs
      (if (not (Variables|Default|GetAirborne))
        (if _up
          (CallFunction|Jump currentInput)
          (elif _lft
            (CallFunction|WalkLeft)
            (elif _rgt
              (CallFunction|WalkRight))))))
    (:then_1
      ;[1 1 1] Collision
      (CallFunction|Collision))
    (:then_2
      ;[1 1 1] "Physics"
      ;;[1 1 1] Add Velocity
      (Transformation|AddWorldOffset (Variables|Default|GetDefaultSceneRoot) (Math|Vector|MakeVector 0.0 (.X (Math|Vector2D|BreakVector2D (Variables|Default|GetVelocity))) (.Y (Math|Vector2D|BreakVector2D (Variables|Default|GetVelocity)))) false false)
      ;;[1 1 1] Decrement Vertical Velocity by Gravity if airborne
      (if (Variables|Default|GetAirborne)
        (Variables|Default|SetVelocity (Math|Vector2D|MakeVector2D (* (.X (Math|Vector2D|BreakVector2D (Variables|Default|GetVelocity))) _air_resistance) (* (+ (.Y (Math|Vector2D|BreakVector2D (Variables|Default|GetVelocity))) (Variables|Default|GetGravity%20Force)) _air_resistance)))
        (else
          ;;[1 1 1] Decrement Horizontal by Gravity if grounded
          (Variables|Default|SetVelocity (Math|Vector2D|MakeVector2D (* (.X (Math|Vector2D|BreakVector2D (Variables|Default|GetVelocity))) (Variables|Default|GetGround%20Friction)) 0.0)))))
    (:then_3
      ;[1 1 1] Facing
      (if (not (Variables|Default|GetAirborne))
        ;;[1 1 1] Check if should be facing Left
        (if (and (> (.y (Transformation|GetActorLocation (Variables|Default|Getopponent))) (.y (Transformation|GetWorldLocation (Variables|BP_FGJ_Character_C|GetDefaultSceneRoot self)))) (Variables|Default|GetFacingRight))
          ;;[1 1 1] Face Left
          (Variables|Default|SetFacingRight false)
          (Transformation|SetActorRelativeRotation "0.000000,90.000000,0.000000")
          (Variables|Default|SetFacingMultiplier 1.0)
          (else
            ;;[1 1 1] Check if should be facing Right
            (if (and (< (.y (Transformation|GetActorLocation (Variables|Default|Getopponent))) (.y (Transformation|GetWorldLocation (Variables|BP_FGJ_Character_C|GetDefaultSceneRoot self)))) (not (Variables|Default|GetFacingRight)))
              ;;[1 1 1] Face Right
              (Variables|Default|SetFacingRight true)
              (Transformation|SetActorRelativeRotation "0.000000,-90.000000,0.000000")
              (Variables|Default|SetFacingMultiplier -1.0))))))))

(event EventSetState
  (params (newState :type FGJ%20Player%20State%20Struct%20Structure))
  (bind (_position _velocity _facingright) (Utilities|Struct|BreakFGJ_Player_StateStruct newState))
  (bind (_x _y) (Math|Vector2D|BreakVector2D _position))
  ;[1 1 1] Set Character State
  (Utilities|FlowControl|Sequence
    (:then_0
      (Transformation|SetWorldLocation (Variables|Default|GetDefaultSceneRoot) (Math|Vector|MakeVector 0.0 _x _y) false true))
    (:then_1
      (Variables|Default|SetVelocity _velocity))
    (:then_2
      (bind _output_get (Variables|Default|SetFacingRight _facingright))
      (if _output_get
        (Transformation|SetActorRelativeRotation "0.000000,-90.000000,0.000000")
        (Variables|Default|SetFacingMultiplier -1.0)
        (else
          (Transformation|SetActorRelativeRotation "0.000000,90.000000,0.000000")
          (Variables|Default|SetFacingMultiplier 1.0))))))

(fn ConstructionScript)

(fn Jump
  (params (Input :type U%20Player%20Input%20Struct%20Structure))
  (bind (_up _dwn _lft _rgt) (Utilities|Struct|BreakUPlayerInputStruct Input))
  (if _lft
    (Variables|Default|SetVelocity (Math|Vector2D|MakeVector2D (Math|Float|SelectFloat (* (Variables|Default|GetBack%20Jump%20Speed) (Variables|Default|GetFacingMultiplier)) (* (Variables|Default|GetForward%20Jump%20Speed) (Variables|Default|GetFacingMultiplier)) (Variables|Default|GetFacingRight)) (Variables|Default|GetJump%20Vertical%20Speed)))
    (Variables|Default|SetAirborne true)
    (elif _rgt
      (Variables|Default|SetVelocity (Math|Vector2D|MakeVector2D (Math|Float|SelectFloat (* (Variables|Default|GetForward%20Jump%20Speed) (Variables|Default|GetFacingMultiplier)) (* (Variables|Default|GetBack%20Jump%20Speed) (Variables|Default|GetFacingMultiplier)) (Variables|Default|GetFacingRight)) (Variables|Default|GetJump%20Vertical%20Speed)))
      (Variables|Default|SetAirborne true)
      (else
        (Variables|Default|SetVelocity (Math|Vector2D|MakeVector2D 0.0 (Variables|Default|GetJump%20Vertical%20Speed)))
        (Variables|Default|SetAirborne true)))))

(fn WalkRight
  (Variables|Default|SetVelocity (Math|Vector2D|MakeVector2D (Math|Float|SelectFloat (* (Variables|Default|GetForward%20Speed) (Variables|Default|GetFacingMultiplier)) (* (Variables|Default|GetBack%20Speed) (Variables|Default|GetFacingMultiplier)) (Variables|Default|GetFacingRight)) 0.0)))

(fn WalkLeft
  (Variables|Default|SetVelocity (Math|Vector2D|MakeVector2D (Math|Float|SelectFloat (* (Variables|Default|GetBack%20Speed) (Variables|Default|GetFacingMultiplier)) (* (Variables|Default|GetForward%20Speed) (Variables|Default|GetFacingMultiplier)) (Variables|Default|GetFacingRight)) 0.0)))

(fn Collision
  (Utilities|FlowControl|Sequence
    (:then_0
      ;[1 1 1] Floor collision
      (for _array_element (Class|PrimitiveComponent|GetOverlappingComponents (Variables|Default|GetFloorCollider))
        (if (Components|ComponentHasTag _array_element "Floor")
          (Variables|Default|SetAirborne false)
          (Variables|Default|SetVelocity (Math|Vector2D|MakeVector2D (.X (Math|Vector2D|BreakVector2D (Variables|Default|GetVelocity))) 0.0))
          (Transformation|SetWorldLocation (Variables|Default|GetDefaultSceneRoot) (Math|Vector|MakeVector 0.0 (.y (Transformation|GetWorldLocation (Variables|Default|GetDefaultSceneRoot))) 0.0) false true))))
    (:then_1
      (for _array_element_2 (Collision|GetOverlappingActors (Variables|Default|GetFloorCollider) "BP_FGJ_Character_C" :!class /Script/Engine.PrimitiveComponent)
        (if (> (.y (Transformation|GetActorLocation (Variables|Default|Getopponent))) (.y (Transformation|GetWorldLocation (Variables|BP_FGJ_Character_C|GetDefaultSceneRoot self))))
          (Variables|Default|SetVelocity (Math|Vector2D|MakeVector2D (+ (.X (Math|Vector2D|BreakVector2D (Variables|Default|GetVelocity))) (* (Variables|Default|GetPushForce) -1.0)) (.Y (Math|Vector2D|BreakVector2D (Variables|Default|GetVelocity)))))
          (else
            (Variables|Default|SetVelocity (Math|Vector2D|MakeVector2D (+ (.X (Math|Vector2D|BreakVector2D (Variables|Default|GetVelocity))) (Variables|Default|GetPushForce)) (.Y (Math|Vector2D|BreakVector2D (Variables|Default|GetVelocity)))))))))))

(fn GetState
  (bind _defaultsceneroot (Variables|Default|GetDefaultSceneRoot))
  (bind _returnvalue (Transformation|GetWorldLocation _defaultsceneroot))
  (return (Utilities|Struct|MakeFGJ_Player_StateStruct (Math|Vector2D|MakeVector2D (.y _returnvalue) (.z _returnvalue)) (Variables|Default|GetVelocity) (Variables|Default|GetFacingRight))))